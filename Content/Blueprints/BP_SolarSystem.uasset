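; Solar system actor that builds a set of planets around its own location when play begins.
; For each PlanetList entry it spawns a BP_Planet offset along X by orbit radius, with that entry's scale.
; It passes orbit, rotation and material data to InitializePlanet, using itself as orbit center, and records planets in SpawnedPlanets.
; Tick loops over that array with an empty body, so this Blueprint moves nothing itself.
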(event EventBeginPlay
  (bind _returnvalue (Transformation|GetActorLocation))
  (for _array_element (Variables|Default|GetPlanetList)
    (bind _returnvalue_2 (Game|SpawnActorfromClass "/Game/BP_Planet.BP_Planet_C" (Math|Transform|MakeTransform (+ (Math|Vector|MakeVector (.OrbitRadius (Utilities|Struct|BreakSTR_PlanetData _array_element)) 0.0 0.0) _returnvalue) "0, 0, 0" (.PlanetScale (Utilities|Struct|BreakSTR_PlanetData _array_element))) "Undefined" "MultiplyWithRoot" 0 2e+01 "2.000000,2.000000,2.000000" 0 0.0 0.0 0.0 "0.000000,0.000000,0.000000" 0))
    (Default|InitializePlanet _returnvalue_2 (.OrbitRadius (Utilities|Struct|BreakSTR_PlanetData _array_element)) (.OrbitSpeed (Utilities|Struct|BreakSTR_PlanetData _array_element)) _returnvalue (.RotationSpeed (Utilities|Struct|BreakSTR_PlanetData _array_element)) (.PlanetMaterial (Utilities|Struct|BreakSTR_PlanetData _array_element)))
    (Utilities|Array|Add (Variables|Default|GetSpawnedPlanets) 0)))

(event Collision|EventActorBeginOverlap
  (params (OtherActor :type Actor%20Object%20Reference)))

(event EventTick
  (params (DeltaSeconds :type Float%20%28single-precision%29))
  (for _array_element (Variables|Default|GetSpawnedPlanets)
    _))

(fn ConstructionScript)