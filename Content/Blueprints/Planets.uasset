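; Base-style planet actor that spins its configurable sphere mesh every tick and can travel along a referenced spline.
; The construction script applies ObjectMesh to the sphere.
; MoveObject plays a timeline scaled by TimeToComplete, mapping its track to distance along the spline to set the actor's location.
; Left and right menu-interact inputs and left mouse click all call PlanetSelected, which is an empty stub here.
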(event Custom|MoveObject
  (bind _spline_to_follow (Variables|Default|GetSpline%20To%20follow))
  (bind _spline (Variables|/Game/Blueprints/Bp_SplinePath.Bp_SplinePath_C|GetSpline _spline_to_follow))
  (Components|Timeline|SetPlayRate (Variables|Default|GetT_Move) (/ 1.0 (Variables|Default|GetTime%20To%20Complete)))
  (bind _move_track (Timeline|T_Move Play)
    (:Update
      (Transformation|SetActorLocationAndRotation (Spline|GetLocationatDistanceAlongSpline _spline (Math|Float|Lerp 0.0 (Spline|GetSplineLength _spline) _move_track) "World") "0, 0, 0"))))

(event Input|EnhancedActionEvents|EnhancedInputActionIA_Menu_Interact_Left_Pressed
  (params (ActionValue :type Boolean) (ElapsedSeconds :type Float%20%28double-precision%29) (TriggeredSeconds :type Float%20%28double-precision%29) (InputAction :type Input%20Action%20Object%20Reference :default "/Game/VRTemplate/Input/Actions/IA_Menu_Interact_Left_Pressed.IA_Menu_Interact_Left_Pressed"))
  (CallFunction|PlanetSelected))

(event Input|EnhancedActionEvents|EnhancedInputActionIA_Menu_Interact_Right_Pressed
  (params (ActionValue :type Boolean) (ElapsedSeconds :type Float%20%28double-precision%29) (TriggeredSeconds :type Float%20%28double-precision%29) (InputAction :type Input%20Action%20Object%20Reference :default "/Game/VRTemplate/Input/Actions/IA_Menu_Interact_Right_Pressed.IA_Menu_Interact_Right_Pressed"))
  (CallFunction|PlanetSelected))

(event EventBeginPlay)

(event Collision|EventActorBeginOverlap
  (params (OtherActor :type Actor%20Object%20Reference)))

(event EventTick
  (params (DeltaSeconds :type Float%20%28single-precision%29))
  (Transformation|AddLocalRotation (Variables|Default|GetSphere) (* "0.000000,20.000000,0.000000" (Utilities|Time|GetWorldDeltaSeconds)) false false))

(event Input|MouseEvents|LeftMouseButton
  (params (Key :type Key%20Structure :default "None"))
  (:Pressed
    (CallFunction|PlanetSelected)))

(fn ConstructionScript
  (Components|StaticMesh|SetStaticMesh (Variables|Default|GetSphere) (Variables|Default|GetObjectMesh)))

(fn PlanetSelected)