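; BP_Planet is a planet actor that circles a center point while spinning on its own axis.
; Each tick it advances an orbit angle, places itself on a flat XY circle using degree-based cosine and sine, and adds yaw to its Sphere component.
; InitializePlanet sets the orbit radius, speed, center, spin rate and sphere material.
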(event EventBeginPlay)

(event Collision|EventActorBeginOverlap
  (params (OtherActor :type Actor%20Object%20Reference)))

(event EventTick
  (params (DeltaSeconds :type Float%20%28single-precision%29))
  (bind _orbitradius (Variables|Default|GetOrbitRadius))
  (bind _output_get (Variables|Default|SetOrbitAngle (+ (Variables|Default|GetOrbitAngle) (* DeltaSeconds (Variables|Default|GetOrbitSpeed)))))
  (Transformation|SetActorLocation (+ (Variables|Default|GetCenterLocation) (Math|Vector|MakeVector (* (Math|Trig|Cos(Degrees) _output_get) _orbitradius) (* (Math|Trig|Sin(Degrees) _output_get) _orbitradius) 0.0)) false false)
  (Transformation|AddLocalRotation (Variables|Default|GetSphere) (Math|Rotator|MakeRotator 0.0 0.0 (* DeltaSeconds (Variables|Default|GetRotationSpeed))) false false))

(fn ConstructionScript)

(fn InitializePlanet
  (params (OrbitRadius :type Float%20%28double-precision%29) (OrbitSpeed :type Float%20%28double-precision%29) (OrbitCenter :type Vector) (RotationSpeed :type Float%20%28double-precision%29) (Material :type Material%20Interface%20Object%20Reference))
  (Variables|Default|SetOrbitRadius OrbitRadius)
  (Variables|Default|SetOrbitSpeed OrbitSpeed)
  (Variables|Default|SetCenterLocation OrbitCenter)
  (Variables|Default|SetRotationSpeed RotationSpeed)
  (Rendering|Material|SetMaterial (Variables|Default|GetSphere) 0 Material))